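; BP_CorruptionZone is a box trigger zone that applies a configurable GameplayEffect to overlapping actors that have a UTHUB_ASC ability system component.
; On begin overlap it stores each returned effect handle in the PlayerEffects map, keyed by actor.
; On end overlap, FindPlayerEffect looks up the component and handle so all stacks of that effect are removed, and the map entry is cleared if removal succeeds.
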(event OnComponentBeginOverlap(Box)
  (params (OverlappedComponent :type Primitive%20Component%20Object%20Reference) (OtherActor :type Actor%20Object%20Reference) (OtherComp :type Primitive%20Component%20Object%20Reference) (OtherBodyIndex :type Integer) (bFromSweep :type Boolean) (SweepResult :type Hit%20Result%20Structure%20%28by%20ref%29))
  (bind _returnvalue (Actor|GetComponentbyClass OtherActor "/Script/UTHUB_GAS2025.UTHUB_ASC"))
  (Utilities|IsValid _returnvalue
    (:Is%20Valid
      (bind _returnvalue_2 (Class|UTHUBASC|ApplyEffectfromClass _returnvalue (Variables|Default|GetGameplayEffect)))
      (Utilities|Map|Add (Variables|Default|GetPlayerEffects) OtherActor _returnvalue_2))))

(event OnComponentEndOverlap(Box)
  (params (OverlappedComponent :type Primitive%20Component%20Object%20Reference) (OtherActor :type Actor%20Object%20Reference) (OtherComp :type Primitive%20Component%20Object%20Reference) (OtherBodyIndex :type Integer))
  (bind (_component _handle _finded_) (CallFunction|FindPlayerEffect OtherActor))
  (if _finded_
    (bind _returnvalue (GameplayEffects|RemoveActiveGameplayEffect _component _handle -1))
    (if _returnvalue
      (Utilities|Map|Remove (Variables|Default|GetPlayerEffects) OtherActor))))

(fn ConstructionScript)

(fn FindPlayerEffect
  (params (Target :type Actor%20Object%20Reference))
  (bind _returnvalue (Actor|GetComponentbyClass Target "/Script/UTHUB_GAS2025.UTHUB_ASC"))
  (bind _playereffects (Variables|Default|GetPlayerEffects))
  (bind (_value _returnvalue_2) (Utilities|Map|Find _playereffects Target))
  (return _returnvalue _value (and _returnvalue_2 (Utilities|IsValid _returnvalue))))