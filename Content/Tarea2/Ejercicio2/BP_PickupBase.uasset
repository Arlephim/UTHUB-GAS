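; BP_PickupBase is a pickup actor that applies a gameplay effect on overlap.
; Its construction script uses the Pickable enum as a row name in DT_Pickups to load PickableInfo and tint the sphere through a dynamic material instance.
; When an overlapping actor has a UTHUB_ASC component, the pickup applies the row's GameplayEffect to it and destroys itself.
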(event OnComponentBeginOverlap(InteractableZone)
  (params (OverlappedComponent :type Primitive%20Component%20Object%20Reference) (OtherActor :type Actor%20Object%20Reference) (OtherComp :type Primitive%20Component%20Object%20Reference) (OtherBodyIndex :type Integer) (bFromSweep :type Boolean) (SweepResult :type Hit%20Result%20Structure%20%28by%20ref%29))
  (bind _returnvalue (Actor|GetComponentbyClass OtherActor "/Script/UTHUB_GAS2025.UTHUB_ASC"))
  (Utilities|IsValid _returnvalue
    (:Is%20Valid
      (Class|UTHUBASC|ApplyEffectfromClass _returnvalue (.gameplayeffect (Variables|Default|GetPickableInfo)))
      (Actor|DestroyActor))))

(fn ConstructionScript
  (bind _sphere (Variables|Default|GetSphere))
  (bind _returnvalue (Utilities|GetDataTableRow "/Game/Tarea2/Ejercicio2/DT_Pickups.DT_Pickups" (Utilities|String|StringToName (Utilities|String|EnumtoString (Variables|Default|GetPickable))))
    (:then
      (Variables|Default|SetPickableInfo _returnvalue)
      (bind _returnvalue_2 (Rendering|Material|CreateDynamicMaterialInstance _sphere 0 "/Game/Tarea2/Ejercicio2/Materials/MI_Pickable.MI_Pickable" "None" :!class /Script/Engine.PrimitiveComponent))
      (Rendering|Material|SetMaterial _sphere 0 _returnvalue_2)
      (Rendering|Material|SetVectorParameterValueonMaterials _sphere "PickableColor" (Math|Conversions|ToVector(LinearColor) (.color (Variables|Default|GetPickableInfo)))))))